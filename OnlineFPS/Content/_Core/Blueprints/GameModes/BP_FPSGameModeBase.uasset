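; Base FPS game mode that registers joining players and handles spawning and possessing their characters.
; PostLogin passes each FPS controller to AddPlayer, and BeginPlay caches all BP_TeamSpawn actors.
; SpawnChara spawns the character at the origin and possesses it, then calls TpToSpawnPoint if the match has started.
; Otherwise, it moves it to a random reachable point around the team spawn indexed by TeamID.
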(event `self.K2_PostLogin`
  (params (NewPlayer :type "PlayerController Object Reference"))
  (bind _asbp_fpsplayer_controller (cast `/Game/_Core/Blueprints/Player/BP_FPSPlayerController` NewPlayer))
  (`self.AddPlayer` _asbp_fpsplayer_controller))

(event `self.ReceiveBeginPlay`
  (bind _outactors (`GameplayStatics.GetAllActorsOfClass` "/Game/_Core/Blueprints/Player/BP_TeamSpawn.BP_TeamSpawn_C"))
  (set `self.TeamSpawns` _outactors))

(event `self.SpawnChara`
  (params (_controller :type "FPSPlayerController Object Reference") (_chara :type "FPSCharacter Class Reference"))
  (`|ExecutionSequence`
    (:`then_0`
      (bind _spawnedchara (`self.SpawnAndPossess` _controller _chara)))
    (:`then_1`
      (if (`self.HasMatchStarted`)
        (`FPSCharacter.TpToSpawnPoint` _spawnedchara)
        (else
          (bind _asfps_player_state (cast `FPS_PlayerState` (`Controller.PlayerState` _controller)))
          (`self.SpawnAtTeamSpawn` _spawnedchara (`FPS_PlayerState.teamID` _asfps_player_state)))))))

(fn `SpawnAndPossess`
  (params (Controller :type "FPSPlayerController Object Reference") (Chara :type "FPSCharacter Class Reference"))
  (returns (SpawnedChara :type "FPSCharacter Object Reference"))
  (bind _asbp_fpsplayer_controller (cast `/Game/_Core/Blueprints/Player/BP_FPSPlayerController` Controller))
  (bind _returnvalue (`|SpawnActorFromClass` Chara (`KismetMathLibrary.MakeTransform` (0.0 0.0 0.0)) "Undefined" "MultiplyWithRoot" null null))
  (`Controller.Possess` _asbp_fpsplayer_controller _returnvalue)
  (return _returnvalue))

(fn `SpawnAtTeamSpawn`
  (params (Chara :type "FPSCharacter Object Reference") (TeamID :type Integer))
  (bind _output (`|GetArrayItem` (`self.TeamSpawns`) TeamID))
  (`self.K2_SetActorLocation` Chara (`NavigationSystemV1.K2_GetRandomReachablePointInRadius` (`self.K2_GetActorLocation` _output) (`/Game/_Core/Blueprints/Player/BP_TeamSpawn.Radius` _output) null null) false false))

(fn `UserConstructionScript`)