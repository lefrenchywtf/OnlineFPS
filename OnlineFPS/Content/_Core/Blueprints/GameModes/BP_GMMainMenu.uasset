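; Main menu game mode that loads player settings, stages preview characters and handles hosting, finding and joining online sessions.
; On BeginPlay it loads or creates the save, copies settings into variables, spawns team-skin characters with the primary gun at menu spawn points, then applies volume and quality.
; Session search filters by a game key to fill the HUD server list.
; Hosting through the GameInstance or joining saves settings first.
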(event `HostGame`
  (params (MapIndex :type Integer) (ModeIndex :type Integer) (MaxPlayers :type Integer))
  (`self.SaveVariables`)
  (`/Game/_Core/Blueprints/BP_FPSGameInstance.HostGame` (`self.GameInstance`) MapIndex ModeIndex MaxPlayers))

(event `self.ReceiveBeginPlay`
  (bind _asbp_fpsgame_instance (cast `/Game/_Core/Blueprints/BP_FPSGameInstance` (`GameplayStatics.GetGameInstance`)))
  (set `self.GameInstance` _asbp_fpsgame_instance)
  (`self.LoadGame`)
  (`self.SetSaveVariables`)
  (`self.SpawnPlayers`)
  (`/Game/_Core/Blueprints/BP_FPSGameInstance.SetVolumes` (`self.GameInstance`) (`self.SaveGame`))
  (`self.SetQuality`))

(event `FindGames`
  (bind _hud (`self.HUD`))
  (bind _results (`FindSessionsCallbackProxyAdvanced.FindSessionsAdvanced` (`GameplayStatics.GetPlayerController` 0) 0 false "ClientServersOnly" (`|MakeArray` (`AdvancedSessionsLibrary.MakeLiteralSessionSearchProperty` (`AdvancedSessionsLibrary.MakeLiteralSessionPropertyString` "MyGame" "FPSOnline2") "Equals")))
    (:`OnSuccess`
      (for _array_element _results
        (`/Game/_Core/HUD/W_MainMenu.AddServer` _hud _array_element))
      (set `WidgetSwitcher.ActiveWidgetIndex` 2 (`/Game/_Core/HUD/W_MainMenu.WidgetSwitcher_136` _hud)))))

(event `JoinSession`
  (params (Session :type "BlueprintSessionResult Structure"))
  (`self.SaveVariables`)
  (`JoinSessionCallbackProxy.JoinSession` (`GameplayStatics.GetPlayerController` 0) Session))

(fn `LoadGame`
  (bind _returnvalue (`GameplayStatics.DoesSaveGameExist` "FPSOnline2"))
  (if _returnvalue
    (bind _returnvalue_2 (`GameplayStatics.LoadGameFromSlot` "FPSOnline2"))
    (bind _asbp_save_game (cast `/Game/_Core/Blueprints/BP_SaveGame` _returnvalue_2))
    (set `self.SaveGame` _asbp_save_game)
    (else
      (bind _returnvalue_3 (`GameplayStatics.CreateSaveGameObject` "/Game/_Core/Blueprints/BP_SaveGame.BP_SaveGame_C"))
      (set `self.SaveGame` _returnvalue_3))))

(fn `SaveVariables`
  (bind _savegame (`self.SaveGame`))
  (set `/Game/_Core/Blueprints/BP_SaveGame.Team Skins` (`self.TeamSkins`) _savegame)
  (set `/Game/_Core/Blueprints/BP_SaveGame.Sensitivity` (`self.Sensitivity`) _savegame)
  (set `/Game/_Core/Blueprints/BP_SaveGame.Guns` (`self.Guns`) _savegame)
  (set `/Game/_Core/Blueprints/BP_SaveGame.ToggleSprint` (`self.ToggleSprint`) _savegame)
  (set `/Game/_Core/Blueprints/BP_SaveGame.ToggleCrouch` (`self.ToggleCrouch`) _savegame)
  (`GameplayStatics.SaveGameToSlot` (`self.SaveGame`) "FPSOnline2"))

(fn `SetQuality`
  (bind _returnvalue (`GameUserSettings.GetGameUserSettings`))
  (`GameUserSettings.SetOverallScalabilityLevel` _returnvalue (`/Game/_Core/Blueprints/BP_SaveGame.OverallQuality` (`self.SaveGame`)))
  (`GameUserSettings.ApplySettings` _returnvalue true))

(fn `SetSaveVariables`
  (set `self.TeamSkins` (`/Game/_Core/Blueprints/BP_SaveGame.Team Skins` (`self.SaveGame`)))
  (set `self.Guns` (`/Game/_Core/Blueprints/BP_SaveGame.Guns` (`self.SaveGame`)))
  (set `self.Sensitivity` (`/Game/_Core/Blueprints/BP_SaveGame.Sensitivity` (`self.SaveGame`)))
  (set `self.ToggleSprint` (`/Game/_Core/Blueprints/BP_SaveGame.ToggleSprint` (`self.SaveGame`)))
  (set `self.ToggleCrouch` (`/Game/_Core/Blueprints/BP_SaveGame.ToggleCrouch` (`self.SaveGame`))))

(fn `SetSensitivity`
  (params (Sensitivity :type "Float (double-precision)"))
  (set `self.Sensitivity` Sensitivity))

(fn `SetToggle`
  (params (`Sprint?` :type Boolean) (NewVal :type Boolean))
  (if `Sprint?`
    (set `self.ToggleSprint` NewVal)
    (else
      (set `self.ToggleCrouch` NewVal))))

(fn `SetVolume`
  (params (Type :type "/Game/_Core/Blueprints/E_VolumeType Enum" :default "NewEnumerator0") (Value :type "Float (double-precision)"))
  (bind _savegame (`self.SaveGame`))
  (bind _value (`local.Value`))
  (switch `/Game/_Core/Blueprints/E_VolumeType` Type
    (:`NewEnumerator0`
      (set `/Game/_Core/Blueprints/BP_SaveGame.MasterVolume` (`local.Value`) (`self.SaveGame`)))
    (:`NewEnumerator1`
      (set `/Game/_Core/Blueprints/BP_SaveGame.SFXVolume` _value _savegame))
    (:`NewEnumerator2`
      (set `/Game/_Core/Blueprints/BP_SaveGame.MusicVolume` _value _savegame))))

(fn `SpawnPlayers`
  (bind _guns_primary (break `PlayerWeapons` (`self.Guns`)))
  (bind _outactors (`GameplayStatics.GetAllActorsOfClass` "/Game/_Core/Blueprints/Player/BP_MenuPlayerSpawn.BP_MenuPlayerSpawn_C"))
  (for (_array_element _array_index) _outactors
    (bind _returnvalue (`|SpawnActorFromClass` (`|GetArrayItem` (`self.TeamSkins`) _array_index) (`self.GetTransform` _array_element) "Undefined" "MultiplyWithRoot" null null))
    (bind _returnvalue_2 (`|SpawnActorFromClass` _guns_primary (`KismetMathLibrary.MakeTransform` (0.0 0.0 0.0)) "Undefined" "MultiplyWithRoot" null null))
    (`self.K2_AttachToComponent` _returnvalue_2 (`Character.Mesh` _returnvalue) "handgrip_r" "SnapToTarget" "SnapToTarget" "SnapToTarget" true)))

(fn `UserConstructionScript`)