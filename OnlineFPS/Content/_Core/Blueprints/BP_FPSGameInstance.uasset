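; Game instance for an online FPS that hosts multiplayer matches and manages sound class volumes.
; HostGame creates an Advanced Session tagged with game, map and mode names, then opens the chosen map as a listen server.
; Init applies the base sound mix after a short delay, and SetVolumes overrides Master, SFX and Music from a save game.
; Shutdown has the main menu game mode save its variables, if active.
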(event `self.ReceiveInit`
  (`KismetSystemLibrary.Delay` 0.1)
  (`GameplayStatics.SetBaseSoundMix` "/Game/_Core/Audio/SM_SoundMix.SM_SoundMix"))

(event `HostGame`
  (params (mapIndex :type Integer) (ModeIndx :type Integer) (MaxPlayers :type Integer))
  (`CreateSessionCallbackProxyAdvanced.CreateAdvancedSession` (`self.SetExtraSettings` mapIndex ModeIndx) (`GameplayStatics.GetPlayerController` 0) MaxPlayers
    (:`OnSuccess`
      (`GameplayStatics.OpenLevelBySoftObjectPtr` (`|GetArrayItem` (`self.Maps`) mapIndex) true (`self.GetModeString` ModeIndx)))))

(event `self.ReceiveShutdown`
  (bind _asbp_gmmain_menu (cast `/Game/_Core/Blueprints/GameModes/BP_GMMainMenu` (`GameplayStatics.GetGameMode`)))
  (`/Game/_Core/Blueprints/GameModes/BP_GMMainMenu.SaveVariables` _asbp_gmmain_menu))

(fn `GetModeString`
  (params (Index :type Integer))
  (returns (ReturnValue :type String))
  (return (`KismetStringLibrary.Concat_StrStr` (`|GetArrayItem` (`self.Modes`) Index) "?listen")))

(fn `SetExtraSettings`
  (params (MapIndex :type Integer) (ModeIndex :type Integer))
  (returns (Array :type "Array of SessionPropertyKeyPair Structure"))
  (return (`|MakeArray` (`AdvancedSessionsLibrary.MakeLiteralSessionPropertyString` "MyGame" "FPSOnline2") (`AdvancedSessionsLibrary.MakeLiteralSessionPropertyString` "MapName" (`|GetArrayItem` (`self.MapName`) MapIndex)) (`AdvancedSessionsLibrary.MakeLiteralSessionPropertyString` "ModeName" (`|GetArrayItem` (`self.ModeName`) ModeIndex)))))

(fn `SetVolumes`
  (params (SaveGame :type "/Game/_Core/Blueprints/BP_SaveGame Object Reference"))
  (`GameplayStatics.SetSoundMixClassOverride` "/Game/_Core/Audio/SM_SoundMix.SM_SoundMix" "/Engine/EngineSounds/Master.Master" (/ (`/Game/_Core/Blueprints/BP_SaveGame.MasterVolume` SaveGame) 100.0))
  (`GameplayStatics.SetSoundMixClassOverride` "/Game/_Core/Audio/SM_SoundMix.SM_SoundMix" "/Engine/EngineSounds/SFX.SFX" (/ (`/Game/_Core/Blueprints/BP_SaveGame.SFXVolume` (`local.SaveGame`)) 100.0))
  (`GameplayStatics.SetSoundMixClassOverride` "/Game/_Core/Audio/SM_SoundMix.SM_SoundMix" "/Engine/EngineSounds/Music.Music" (/ (`/Game/_Core/Blueprints/BP_SaveGame.MusicVolume` (`local.SaveGame`)) 100.0)))