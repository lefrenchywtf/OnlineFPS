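; Player controller for the main menu that sets up input and shows the menu UI.
; On BeginPlay it adds IMC_Player and registers it with Enhanced Input user settings if it is not already registered.
; It then creates W_MainMenu, shows the mouse cursor, and cross-links the widget with BP_GMMainMenu so each holds a reference to the other.
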(event `self.ReceiveBeginPlay`
  (bind _returnvalue (pcsubsystem `EnhancedInputLocalPlayerSubsystem` self))
  (bind _returnvalue_2 (`EnhancedInputSubsystemInterface.GetUserSettings` _returnvalue))
  (`EnhancedInputSubsystemInterface.AddMappingContext` _returnvalue "/Game/_Core/Inputs/IMC_Player.IMC_Player" 0 (struct))
  (if (not (`EnhancedInputUserSettings.IsMappingContextRegistered` _returnvalue_2 "/Game/_Core/Inputs/IMC_Player.IMC_Player"))
    (`EnhancedInputUserSettings.RegisterInputMappingContext` _returnvalue_2 "/Game/_Core/Inputs/IMC_Player.IMC_Player"))
  (bind _returnvalue_3 (`|CreateWidget` "/Game/_Core/HUD/W_MainMenu.W_MainMenu_C" self))
  (bind _output_get (set `self.HUD` _returnvalue_3))
  (`UserWidget.AddToViewport` _output_get 0)
  (set `self.bShowMouseCursor` true)
  (bind _asbp_gmmain_menu (cast `/Game/_Core/Blueprints/GameModes/BP_GMMainMenu` (`GameplayStatics.GetGameMode`)))
  (bind _output_get_2 (set `self.GameMode` _asbp_gmmain_menu))
  (bind _output_get_3 (set `/Game/_Core/Blueprints/GameModes/BP_GMMainMenu.HUD` (`self.HUD`) _output_get_2))
  (set `/Game/_Core/HUD/W_MainMenu.GameMode` _output_get_2 _output_get_3))

(fn `UserConstructionScript`)