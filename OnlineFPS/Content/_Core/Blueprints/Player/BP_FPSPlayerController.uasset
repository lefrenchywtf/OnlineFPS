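; Player controller for a multiplayer FPS, handling input, local UI, saved preferences and team selection.
; On local BeginPlay it adds the input mapping, creates HUD and pause widgets, and loads loadout, skins and settings from the save.
; Enhanced Input actions forward to the possessed character, with optional sprint and crouch toggles.
; Team picks route through a server event to the game mode, while a separate game-mode HUD displays kills, objectives and results.
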(event `self.AddKillToFeed`
  (params (_killer :type "FPSCharacter Object Reference") (_victim :type "FPSCharacter Object Reference") (_gunName :type String))
  (bind _asbp_fps_player_state (cast `/Game/_Core/Blueprints/Player/BP_FPS_PlayerState` (`Pawn.PlayerState` _killer)))
  (bind _asbp_fps_player_state_2 (cast `/Game/_Core/Blueprints/Player/BP_FPS_PlayerState` (`Pawn.PlayerState` _victim)))
  (`/Game/_Core/HUD/W_GameHud.AddAKillToFeed` (`self.GameHud`) _asbp_fps_player_state _asbp_fps_player_state_2 _gunName))

(event `self.UpdateGamemodeHud`
  (`KismetSystemLibrary.Delay` 0.2)
  (`/Game/_Core/HUD/W_GameHud.UpdateObjectives` (`self.GameHud`)))

(event `self.CreateGamemodeWidget`
  (params (_widget :type "UserWidget Class Reference"))
  (bind _returnvalue (`|CreateWidget` _widget self))
  (bind _asw_game_hud (cast `/Game/_Core/HUD/W_GameHud` _returnvalue))
  (bind _output_get (set `self.GameHud` _asw_game_hud))
  (`UserWidget.AddToViewport` _output_get 0))

(event `self.ReceiveBeginPlay`
  (if (`self.IsLocalPlayerController` self)
    (`EnhancedInputSubsystemInterface.AddMappingContext` (pcsubsystem `EnhancedInputLocalPlayerSubsystem` self) "/Game/_Core/Inputs/IMC_Player.IMC_Player" 0 (struct))
    (bind _returnvalue (`|CreateWidget` "/Game/_Core/HUD/W_PlayerHud.W_PlayerHud_C" self))
    (bind _output_get (set `self.PlayerHUD` _returnvalue))
    (`UserWidget.AddToViewport` _output_get 0)
    (`self.Load Game`)
    (`self.SetVariables`)
    (`self.ShowPlayerHUD` false)
    (`self.ShowMouseCursor` true)
    (bind _returnvalue_2 (`|CreateWidget` "/Game/_Core/HUD/W_PauseMenu.W_PauseMenu_C" self))
    (bind _output_get_2 (set `self.PauseMenu` _returnvalue_2))
    (`UserWidget.AddToViewport` _output_get_2 0)))

(event `SelectTeam`
  (params (TeamId :type Integer))
  (`self.Server_SelectTeam` TeamId (`self.TeamSkins`))
  (`self.ShowMouseCursor` false))

(event `EnhancedInput|/Game/_Core/Inputs/InputActions/IA_Move`
  (params (ActionValue :type "Vector2D Structure") (ElapsedSeconds :type "Float (double-precision)") (TriggeredSeconds :type "Float (double-precision)") (InputAction :type "InputAction Object Reference" :default "/Game/_Core/Inputs/InputActions/IA_Move.IA_Move"))
  (bind _chara (`self.Chara`))
  (:`Triggered`
    (`/Engine/EditorBlueprintResources/StandardMacros.IsValid` _chara
      (:`Is Valid`
        (`FPSCharacter.Move` _chara ActionValue))))
  (:`Completed`
    (`/Engine/EditorBlueprintResources/StandardMacros.IsValid` _chara
      (:`Is Valid`
        (`FPSCharacter.SprintChara` _chara false)))))

(event `Server_SelectTeam`
  (params (TeamID :type Integer) (TeamSkins :type "Array of /Game/_Core/Blueprints/Player/BP_FPSCharacter Class Reference"))
  (bind _asbp_fpsgame_mode_base (cast `/Game/_Core/Blueprints/GameModes/BP_FPSGameModeBase` (`GameplayStatics.GetGameMode`)))
  (`FPSGameModeBase.SelectTeam` _asbp_fpsgame_mode_base self TeamID TeamSkins))

(event `EnhancedInput|/Game/_Core/Inputs/InputActions/IA_Jump`
  (params (ActionValue :type Boolean) (ElapsedSeconds :type "Float (double-precision)") (TriggeredSeconds :type "Float (double-precision)") (InputAction :type "InputAction Object Reference" :default "/Game/_Core/Inputs/InputActions/IA_Jump.IA_Jump"))
  (bind _chara (`self.Chara`))
  (:`Triggered`
    (`/Engine/EditorBlueprintResources/StandardMacros.IsValid` _chara
      (:`Is Valid`
        (`FPSCharacter.JumpChara` _chara)))))

(event `EnhancedInput|/Game/_Core/Inputs/InputActions/IA_Sprint`
  (params (ActionValue :type Boolean) (ElapsedSeconds :type "Float (double-precision)") (TriggeredSeconds :type "Float (double-precision)") (InputAction :type "InputAction Object Reference" :default "/Game/_Core/Inputs/InputActions/IA_Sprint.IA_Sprint"))
  (bind _chara (`self.Chara`))
  (bind _chara_2 (`self.Chara`))
  (:`Triggered`
    (`/Engine/EditorBlueprintResources/StandardMacros.IsValid` _chara
      (:`Is Valid`
        (if (`self.bIsSprintToggle`)
          (if (and (`self.bIsSprintToggle`) ActionValue)
            (`FPSCharacter.SprintChara` _chara_2 (not (`FPSCharacter.bIsSprinting` _chara_2))))
          (else
            (`FPSCharacter.SprintChara` _chara ActionValue)))))))

(event `EnhancedInput|/Game/_Core/Inputs/InputActions/IA_Camera`
  (params (ActionValue :type "Vector2D Structure") (ElapsedSeconds :type "Float (double-precision)") (TriggeredSeconds :type "Float (double-precision)") (InputAction :type "InputAction Object Reference" :default "/Game/_Core/Inputs/InputActions/IA_Camera.IA_Camera"))
  (bind _chara (`self.Chara`))
  (:`Triggered`
    (`/Engine/EditorBlueprintResources/StandardMacros.IsValid` _chara
      (:`Is Valid`
        (`FPSCharacter.MoveCamera` _chara ActionValue)))))

(event `EnhancedInput|/Game/_Core/Inputs/InputActions/IA_Crouch`
  (params (ActionValue :type Boolean) (ElapsedSeconds :type "Float (double-precision)") (TriggeredSeconds :type "Float (double-precision)") (InputAction :type "InputAction Object Reference" :default "/Game/_Core/Inputs/InputActions/IA_Crouch.IA_Crouch"))
  (bind _biscrouchtoggle (`self.bIsCrouchToggle`))
  (bind _chara (`self.Chara`))
  (bind _chara_2 (`self.Chara`))
  (:`Triggered`
    (`/Engine/EditorBlueprintResources/StandardMacros.IsValid` _chara_2
      (:`Is Valid`
        (if _biscrouchtoggle
          (if (and _biscrouchtoggle ActionValue)
            (`FPSCharacter.CrouchChara` _chara (not (`Character.bIsCrouched` _chara))))
          (else
            (`FPSCharacter.CrouchChara` _chara_2 ActionValue)))))))

(event `EnhancedInput|/Game/_Core/Inputs/InputActions/IA_ShootGun`
  (params (ActionValue :type Boolean) (ElapsedSeconds :type "Float (double-precision)") (TriggeredSeconds :type "Float (double-precision)") (InputAction :type "InputAction Object Reference" :default "/Game/_Core/Inputs/InputActions/IA_ShootGun.IA_ShootGun"))
  (bind _chara (`self.Chara`))
  (:`Started`
    (`/Engine/EditorBlueprintResources/StandardMacros.IsValid` _chara
      (:`Is Valid`
        (`FPSCharacter.ShootGun` _chara))))
  (:`Completed`
    (`/Engine/EditorBlueprintResources/StandardMacros.IsValid` _chara
      (:`Is Valid`
        (`FPSCharacter.StopShooting` _chara)))))

(event `EnhancedInput|/Game/_Core/Inputs/InputActions/IA_Pause`
  (params (ActionValue :type Boolean) (ElapsedSeconds :type "Float (double-precision)") (TriggeredSeconds :type "Float (double-precision)") (InputAction :type "InputAction Object Reference" :default "/Game/_Core/Inputs/InputActions/IA_Pause.IA_Pause"))
  (:`Started`
    (`self.ShowPause`)))

(event `EnhancedInput|/Game/_Core/Inputs/InputActions/IA_EquipPrimary`
  (params (ActionValue :type Boolean) (ElapsedSeconds :type "Float (double-precision)") (TriggeredSeconds :type "Float (double-precision)") (InputAction :type "InputAction Object Reference" :default "/Game/_Core/Inputs/InputActions/IA_EquipPrimary.IA_EquipPrimary"))
  (bind _chara (`self.Chara`))
  (:`Triggered`
    (`/Engine/EditorBlueprintResources/StandardMacros.IsValid` _chara
      (:`Is Valid`
        (`FPSCharacter.EquipGun` _chara "PRIMARY")))))

(event `EnhancedInput|/Game/_Core/Inputs/InputActions/IA_EquipSecondary`
  (params (ActionValue :type Boolean) (ElapsedSeconds :type "Float (double-precision)") (TriggeredSeconds :type "Float (double-precision)") (InputAction :type "InputAction Object Reference" :default "/Game/_Core/Inputs/InputActions/IA_EquipSecondary.IA_EquipSecondary"))
  (bind _chara (`self.Chara`))
  (:`Triggered`
    (`/Engine/EditorBlueprintResources/StandardMacros.IsValid` _chara
      (:`Is Valid`
        (`FPSCharacter.EquipGun` _chara "SECONDARY")))))

(event `EnhancedInput|/Game/_Core/Inputs/InputActions/IA_ADS`
  (params (ActionValue :type Boolean) (ElapsedSeconds :type "Float (double-precision)") (TriggeredSeconds :type "Float (double-precision)") (InputAction :type "InputAction Object Reference" :default "/Game/_Core/Inputs/InputActions/IA_ADS.IA_ADS"))
  (bind _chara (`self.Chara`))
  (bind _chara_2 (`self.Chara`))
  (:`Started`
    (`/Engine/EditorBlueprintResources/StandardMacros.IsValid` _chara_2
      (:`Is Valid`
        (`FPSCharacter.StartADS` _chara_2))))
  (:`Canceled`
    (`/Engine/EditorBlueprintResources/StandardMacros.IsValid` _chara :!label _label
      (:`Is Valid`
        (`FPSCharacter.EndADS` _chara))))
  (:`Completed`
    (goto _label)))

(event `EnhancedInput|/Game/_Core/Inputs/InputActions/IA_ReloadGun`
  (params (ActionValue :type Boolean) (ElapsedSeconds :type "Float (double-precision)") (TriggeredSeconds :type "Float (double-precision)") (InputAction :type "InputAction Object Reference" :default "/Game/_Core/Inputs/InputActions/IA_ReloadGun.IA_ReloadGun"))
  (bind _chara (`self.Chara`))
  (:`Triggered`
    (`/Engine/EditorBlueprintResources/StandardMacros.IsValid` _chara
      (:`Is Valid`
        (`FPSCharacter.StartReloading` _chara)))))

(event `self.HidePreGameCounter`
  (`Widget.SetVisibility` (`/Game/_Core/HUD/W_GameHud.PregameCount` (`self.GameHud`)) "Hidden"))

(event `self.ShowPlayerHUD`
  (params (_bShow :type Boolean))
  (if _bShow
    (`Widget.SetVisibility` (`self.PlayerHUD`) "HitTestInvisible")
    (else
      (`Widget.SetVisibility` (`self.PlayerHUD`) "Hidden"))))

(event `self.ShowMouseCursor`
  (params (_bShow :type Boolean))
  (bind _output_get (set `self.bShowMouseCursor` _bShow))
  (if _output_get
    (`WidgetBlueprintLibrary.SetInputMode_UIOnlyEx` self null)
    (else
      (`WidgetBlueprintLibrary.SetInputMode_GameOnly` self))))

(fn `EndOfGameDisplay`
  (params (Victory :type Boolean))
  (`Widget.SetVisibility` (`self.PlayerHUD`) "Hidden")
  (`/Game/_Core/HUD/W_GameHud.DisplayEndOfGame` (`self.GameHud`) Victory))

(fn `Load Game`
  (bind _returnvalue (`GameplayStatics.DoesSaveGameExist` "FPSOnline2"))
  (if _returnvalue
    (bind _returnvalue_2 (`GameplayStatics.LoadGameFromSlot` "FPSOnline2"))
    (bind _asbp_save_game (cast `/Game/_Core/Blueprints/BP_SaveGame` _returnvalue_2))
    (set `self.SaveGame` _asbp_save_game)))

(fn `SetPlayerName`)

(fn `SetVariables`
  (set `self.TeamSkins` (`/Game/_Core/Blueprints/BP_SaveGame.Team Skins` (`self.SaveGame`)))
  (set `self.Guns` (`/Game/_Core/Blueprints/BP_SaveGame.Guns` (`self.SaveGame`)))
  (set `self.Sensitivity` (`/Game/_Core/Blueprints/BP_SaveGame.Sensitivity` (`self.SaveGame`)))
  (set `self.bIsSprintToggle` (`/Game/_Core/Blueprints/BP_SaveGame.ToggleSprint` (`self.SaveGame`)))
  (set `self.bIsCrouchToggle` (`/Game/_Core/Blueprints/BP_SaveGame.ToggleCrouch` (`self.SaveGame`)))
  (set `self.savedFOV` (`/Game/_Core/Blueprints/BP_SaveGame.FOV` (`self.SaveGame`))))

(fn `ShowPause`
  (if (`|EnumEquality` (`Widget.Visibility` (`self.PauseMenu`)) "Visible")
    (`Widget.SetVisibility` (`self.PauseMenu`) "Hidden")
    (set `self.bShowMouseCursor` false)
    (`WidgetBlueprintLibrary.SetInputMode_GameOnly` self)
    (else
      (`Widget.SetVisibility` (`self.PauseMenu`) "Visible")
      (set `self.bShowMouseCursor` true))))

(fn `UserConstructionScript`)