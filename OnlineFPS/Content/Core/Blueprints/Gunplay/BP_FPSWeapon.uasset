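; BP_FPSWeapon is a weapon actor that binds itself to an owning FPS character.
; SetWeaponOwner stores the owner, caches its camera and registers the weapon in the primary or secondary slot by its type, then calls AttachWeapon.
; AttachWeapon snaps it to the right-hand grip socket, using the first-person mesh when the owner is locally controlled and the character's main mesh otherwise.
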(fn `AttachWeapon`
  (bind _weaponowner (`self.weaponOwner`))
  (bind _asbp_fpscharacter (cast `/Game/Core/Blueprints/Player/BP_FPSCharacter` _weaponowner))
  (if (`Pawn.IsLocallyControlled` _weaponowner)
    (`self.K2_AttachToComponent` (`/Game/Core/Blueprints/Player/BP_FPSCharacter.FPP_Mesh` _asbp_fpscharacter) "handGrip_r" "SnapToTarget" "SnapToTarget" "SnapToTarget")
    (else
      (`self.K2_AttachToComponent` (`Character.Mesh` _asbp_fpscharacter) "handGrip_r" "SnapToTarget" "SnapToTarget" "SnapToTarget"))))

(fn `GetPlayerCamera`
  (params (Chara :type "FPSCharacter Object Reference"))
  (bind _asbp_fpscharacter (cast `/Game/Core/Blueprints/Player/BP_FPSCharacter` Chara))
  (set `self.playerCamera` (`/Game/Core/Blueprints/Player/BP_FPSCharacter.Camera` _asbp_fpscharacter)))

(fn `SetWeaponOwner`
  (params (Character :type "FPSCharacter Object Reference"))
  (bind _output_get (set `self.weaponOwner` Character))
  (`self.GetPlayerCamera` _output_get)
  (switch `EWeaponType` (`self.Type`)
    (:`PRIMARY`
      (set `FPSCharacter.primaryWeapon` self _output_get))
    (:`SECONDARY`
      (set `FPSCharacter.secondaryWeapon` self _output_get)))
  (`self.AttachWeapon`))

(fn `UserConstructionScript`)