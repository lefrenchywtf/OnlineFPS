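; First-person shooter player controller that turns Enhanced Input actions into commands on its character reference, Chara.
; On BeginPlay, the local controller adds the IMC_Player mapping context.
; Each action checks Chara is valid, then calls its function for movement, camera, jump, crouch, sprint toggle, shooting start and stop, or primary and secondary weapon equipping.
; The gameplay logic itself lives in the character.
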(event `self.ReceiveBeginPlay`
  (if (`self.IsLocalPlayerController` self)
    (`EnhancedInputSubsystemInterface.AddMappingContext` (pcsubsystem `EnhancedInputLocalPlayerSubsystem` self) "/Game/Core/Inputs/IMC_Player.IMC_Player" 0 (struct))))

(event `EnhancedInput|/Game/Core/Inputs/InputActions/IA_Move`
  (params (ActionValue :type "Vector2D Structure") (ElapsedSeconds :type "Float (double-precision)") (TriggeredSeconds :type "Float (double-precision)") (InputAction :type "InputAction Object Reference" :default "/Game/Core/Inputs/InputActions/IA_Move.IA_Move"))
  (bind _chara (`self.Chara`))
  (:`Triggered`
    (`/Engine/EditorBlueprintResources/StandardMacros.IsValid` _chara
      (:`Is Valid`
        (`FPSCharacter.Move` _chara ActionValue)))))

(event `EnhancedInput|/Game/Core/Inputs/InputActions/IA_Jump`
  (params (ActionValue :type Boolean) (ElapsedSeconds :type "Float (double-precision)") (TriggeredSeconds :type "Float (double-precision)") (InputAction :type "InputAction Object Reference" :default "/Game/Core/Inputs/InputActions/IA_Jump.IA_Jump"))
  (bind _chara (`self.Chara`))
  (:`Triggered`
    (`/Engine/EditorBlueprintResources/StandardMacros.IsValid` _chara
      (:`Is Valid`
        (`FPSCharacter.JumpChara` _chara)))))

(event `EnhancedInput|/Game/Core/Inputs/InputActions/IA_Crouch`
  (params (ActionValue :type Boolean) (ElapsedSeconds :type "Float (double-precision)") (TriggeredSeconds :type "Float (double-precision)") (InputAction :type "InputAction Object Reference" :default "/Game/Core/Inputs/InputActions/IA_Crouch.IA_Crouch"))
  (bind _chara (`self.Chara`))
  (:`Triggered`
    (`/Engine/EditorBlueprintResources/StandardMacros.IsValid` _chara
      (:`Is Valid`
        (`FPSCharacter.CrouchChara` _chara ActionValue)))))

(event `EnhancedInput|/Game/Core/Inputs/InputActions/IA_Camera`
  (params (ActionValue :type "Vector2D Structure") (ElapsedSeconds :type "Float (double-precision)") (TriggeredSeconds :type "Float (double-precision)") (InputAction :type "InputAction Object Reference" :default "/Game/Core/Inputs/InputActions/IA_Camera.IA_Camera"))
  (bind _chara (`self.Chara`))
  (:`Triggered`
    (`/Engine/EditorBlueprintResources/StandardMacros.IsValid` _chara
      (:`Is Valid`
        (`FPSCharacter.MoveCamera` _chara ActionValue)))))

(event `EnhancedInput|/Game/Core/Inputs/InputActions/IA_Sprint`
  (params (ActionValue :type Boolean) (ElapsedSeconds :type "Float (double-precision)") (TriggeredSeconds :type "Float (double-precision)") (InputAction :type "InputAction Object Reference" :default "/Game/Core/Inputs/InputActions/IA_Sprint.IA_Sprint"))
  (bind _chara (`self.Chara`))
  (:`Triggered`
    (`/Engine/EditorBlueprintResources/StandardMacros.IsValid` _chara
      (:`Is Valid`
        (`FPSCharacter.SprintChara` _chara (not (`FPSCharacter.bIsSprinting` _chara)))))))

(event `EnhancedInput|/Game/Core/Inputs/InputActions/IA_ShootGun`
  (params (ActionValue :type Boolean) (ElapsedSeconds :type "Float (double-precision)") (TriggeredSeconds :type "Float (double-precision)") (InputAction :type "InputAction Object Reference" :default "/Game/Core/Inputs/InputActions/IA_ShootGun.IA_ShootGun"))
  (bind _chara (`self.Chara`))
  (:`Started`
    (`/Engine/EditorBlueprintResources/StandardMacros.IsValid` _chara
      (:`Is Valid`
        (`FPSCharacter.ShootGun` _chara))))
  (:`Completed`
    (`/Engine/EditorBlueprintResources/StandardMacros.IsValid` _chara
      (:`Is Valid`
        (`FPSCharacter.StopShooting` _chara)))))

(event `EnhancedInput|/Game/Core/Inputs/InputActions/IA_EquipPrimary`
  (params (ActionValue :type Boolean) (ElapsedSeconds :type "Float (double-precision)") (TriggeredSeconds :type "Float (double-precision)") (InputAction :type "InputAction Object Reference" :default "/Game/Core/Inputs/InputActions/IA_EquipPrimary.IA_EquipPrimary"))
  (bind _chara (`self.Chara`))
  (:`Triggered`
    (`/Engine/EditorBlueprintResources/StandardMacros.IsValid` _chara
      (:`Is Valid`
        (`FPSCharacter.EquipGun` _chara "PRIMARY")))))

(event `EnhancedInput|/Game/Core/Inputs/InputActions/IA_EquipSecondary`
  (params (ActionValue :type Boolean) (ElapsedSeconds :type "Float (double-precision)") (TriggeredSeconds :type "Float (double-precision)") (InputAction :type "InputAction Object Reference" :default "/Game/Core/Inputs/InputActions/IA_EquipSecondary.IA_EquipSecondary"))
  (bind _chara (`self.Chara`))
  (:`Triggered`
    (`/Engine/EditorBlueprintResources/StandardMacros.IsValid` _chara
      (:`Is Valid`
        (`FPSCharacter.EquipGun` _chara "SECONDARY")))))

(fn `UserConstructionScript`)